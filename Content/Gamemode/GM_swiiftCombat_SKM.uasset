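; Game mode Blueprint for the swiiftCombat SKM variant in Mordhau that applies equipment and perk bans to the match.
; One second after BeginPlay, it casts the game state to MordhauGameState and copies its own BannedEquipment and BannedPerks into it.
; Tick is disabled and the construction script only calls its parent.
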(event EventBeginPlay
  (|CallParentFunction)
  (Utilities|FlowControl|Delay 1.0)
  (bind _asmordhau_game_state (Utilities|Casting|CastToMordhauGameState (Game|GetGameState)))
  (Variables|/Script/Mordhau.MordhauGameState|SetBannedEquipment _asmordhau_game_state (Variables|Default|GetBanned%20Equipment))
  (Variables|/Script/Mordhau.MordhauGameState|SetBannedPerks _asmordhau_game_state (Variables|Default|GetBanned%20Perks)))

(event EventTick
  (params (DeltaSeconds :type Float%20%28single-precision%29))
  (|CallParentFunction DeltaSeconds) ; This node is disabled and will not be called.\nDrag off pins to build functionality.
)

(fn ConstructionScript
  (|CallParentFunction))