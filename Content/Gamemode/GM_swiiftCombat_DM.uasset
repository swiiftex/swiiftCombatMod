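; Deathmatch game mode for swiiftCombat in Mordhau that rewards kills with restored health and stamina.
; Shortly after BeginPlay it copies its banned equipment and perk lists to the MordhauGameState, then spawns and stores a BP_swiiftEquipmentRemapper.
; On each kill, it runs the parent logic, then replicates a health and stamina boost to the killer's controlled MordhauCharacter.
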(event EventBeginPlay
  (|CallParentFunction)
  (Utilities|FlowControl|Delay 1.0)
  (bind _asmordhau_game_state (Utilities|Casting|CastToMordhauGameState (Game|GetGameState)))
  (Variables|/Script/Mordhau.MordhauGameState|SetBannedEquipment _asmordhau_game_state (Variables|Default|GetBanned%20Equipment))
  (Variables|/Script/Mordhau.MordhauGameState|SetBannedPerks _asmordhau_game_state (Variables|Default|GetBanned%20Perks))
  (bind _returnvalue (Game|SpawnActorfromClass "/swiiftCombatMod/BP_swiiftEquipmentRemapper.BP_swiiftEquipmentRemapper_C" (Math|Transform|MakeTransform "0, 0, 0") "Undefined" 0 0))
  (Variables|Default|SetEquipment%20Remapper _returnvalue))

(event EventTick
  (params (DeltaSeconds :type Float%20%28single-precision%29))
  (|CallParentFunction DeltaSeconds) ; This node is disabled and will not be called.\nDrag off pins to build functionality.
)

(event EventOnKilled
  (params (Killer :type Controller%20Object%20Reference) (KilledPlayer :type Controller%20Object%20Reference) (KilledPawn :type Pawn%20Object%20Reference) (Type :type EMordhauDamageType%20Enum :default "Generic") (SubType :type Byte :default 0) (DamageSource :type Actor%20Object%20Reference) (DamageAgent :type Actor%20Object%20Reference))
  (|CallParentFunction Killer KilledPlayer KilledPawn Type SubType DamageSource DamageAgent)
  (bind _asmordhau_character (Utilities|Casting|CastToMordhauCharacter (Pawn|GetControlledPawn Killer)))
  (Class|AdvancedCharacter|OffsetHealth _asmordhau_character 100 true)
  (Class|MordhauCharacter|OffsetStamina _asmordhau_character 100 true))

(fn ConstructionScript
  (|CallParentFunction))